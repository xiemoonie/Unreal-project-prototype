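; BP_HealingItem is a health pickup that heals the player when touched.
; Each tick it rotates the actor by adding a fixed roll step to the box component's relative rotation, so it spins.
; When a BP_MyPlayerShooter overlaps the box, it plays a thud sound, calls Healing on player pawn 0's Health component and destroys itself.
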(event `self.ReceiveTick`
  (params (DeltaSeconds :type "Float (single-precision)"))
  (bind (_relativerotation_roll _relativerotation_pitch _relativerotation_yaw) (`KismetMathLibrary.BreakRotator` (`SceneComponent.RelativeRotation` (`self.BoxComp`))))
  (`self.K2_SetActorRotation` (`KismetMathLibrary.MakeRotator` (+ _relativerotation_roll 2.0) _relativerotation_pitch _relativerotation_yaw)))

(event `self.BoxComp.OnComponentBeginOverlap`
  (params (OverlappedComponent :type "PrimitiveComponent Object Reference") (OtherActor :type "Actor Object Reference") (OtherComp :type "PrimitiveComponent Object Reference") (OtherBodyIndex :type Integer) (bFromSweep :type Boolean) (SweepResult :type "HitResult Structure (by ref)"))
  (if (== (`GameplayStatics.GetObjectClass` OtherActor) "/Game/Assets/Blueprint/BP_MyPlayerShooter.BP_MyPlayerShooter_C")
    (`GameplayStatics.PlaySound2D` "/Game/Assets/Audio/Thud_Audio.Thud_Audio" 1.0 1.0 0.0 null null)
    (bind _asbp_my_player_shooter (cast `/Game/Assets/Blueprint/BP_MyPlayerShooter` (`GameplayStatics.GetPlayerPawn` 0)))
    (`Health.Healing` (`/Game/Assets/Blueprint/BP_MyPlayerShooter.Health` _asbp_my_player_shooter))
    (`self.K2_DestroyActor`)))

(fn `UserConstructionScript`)