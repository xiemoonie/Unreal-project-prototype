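; BP_Mover is a trigger-driven actor that pairs a Trigger with a Mover and lights up when the matching grabbable object touches it.
; On BeginPlay it passes the Mover to the Trigger, leaving any movement logic to those components.
; On Trigger overlap, a BP_Grabbable tagged with the Trigger's ObjetoGrabbable value switches the static mesh to an emissive material, with no revert in this graph.
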(event `self.ReceiveBeginPlay`
  (`TriggerComponent.SetMover` (`self.Trigger`) (`self.Mover`)))

(event `self.Trigger.OnComponentBeginOverlap`
  (params (OverlappedComponent :type "PrimitiveComponent Object Reference") (OtherActor :type "Actor Object Reference") (OtherComp :type "PrimitiveComponent Object Reference") (OtherBodyIndex :type Integer) (bFromSweep :type Boolean) (SweepResult :type "HitResult Structure (by ref)"))
  (if (== (`GameplayStatics.GetObjectClass` OtherActor) "/Game/Assets/Blueprint/BP_Grabbable.BP_Grabbable_C")
    (bind _asbp_grabbable (cast `/Game/Assets/Blueprint/BP_Grabbable` OtherActor))
    (if (`KismetArrayLibrary.Array_Contains` (`Actor.Tags` _asbp_grabbable) (`TriggerComponent.ObjetoGrabbable` (`self.Trigger`)))
      (`PrimitiveComponent.SetMaterial` (`self.StaticMeshComponent`) 0 "/Game/Assets/Materials/M_EmissiveBase.M_EmissiveBase"))))

(fn `UserConstructionScript`)