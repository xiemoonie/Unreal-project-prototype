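; BP_MyPlayerShooter is the player Blueprint that shows a health bar and handles grab input.
; On BeginPlay it creates WBP_HealthBar and adds it to the viewport, except in MainMenuMap.
; Tick copies the Health component's current value into the created widget's HealthPercentage every frame, with no check that the widget exists.
; Pressing and releasing the Grab input calls Grab and Release on the Grabber.
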(event `self.ReceiveBeginPlay`
  (bind _returnvalue (`GameplayStatics.GetCurrentLevelName` true))
  (if (`KismetStringLibrary.NotEqual_StrStr` _returnvalue "MainMenuMap")
    (bind _returnvalue_2 (`|CreateWidget` "/Game/Assets/Blueprint/Widgets/WBP_HealthBar.WBP_HealthBar_C"))
    (bind _output_get (set `self.HealthBarWidget` _returnvalue_2))
    (`UserWidget.AddToViewport` _output_get 0)))

(event `self.ReceiveTick`
  (params (DeltaSeconds :type "Float (single-precision)"))
  (bind _returnvalue (`Health.GetCurrentHealth` (`self.Health`)))
  (set `/Game/Assets/Blueprint/Widgets/WBP_HealthBar.HealthPercentage` _returnvalue (stale `self.ReceiveBeginPlay` _returnvalue_2)))

(event `InputAction|Grab`
  (params (Key :type "Key Structure"))
  (:`Pressed`
    (`Grabber.Grab` (`self.Grabber`)))
  (:`Released`
    (`Grabber.Release` (`self.Grabber`))))

(fn `UserConstructionScript`)